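; Base passive Gameplay Ability that keeps a gameplay effect on its owner while the ability is active.
; On activation it builds a spec from the GameplayEffectClass variable and applies it to the owner's Ability System Component.
; When the ability ends it removes all stacks of that effect class from the same component.
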(event `self.K2_ActivateAbility`
  (`self.ApplyGE`))

(event `self.K2_OnEndAbility`
  (params (bWasCancelled :type Boolean))
  (`self.RemoveGE`))

(fn `ApplyGE`
  (bind _returnvalue (`self.GetAbilitySystemComponentFromActorInfo`))
  (`AbilitySystemComponent.BP_ApplyGameplayEffectSpecToSelf` _returnvalue (`AbilitySystemComponent.MakeOutgoingSpec` :`self` _returnvalue :`GameplayEffectClass` (`self.Gameplay Effect Class`))))

(fn `RemoveGE`
  (`AbilitySystemComponent.RemoveActiveGameplayEffectBySourceEffect` (`self.GetAbilitySystemComponentFromActorInfo`) (`self.Gameplay Effect Class`) null -1))