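; GA_FireBolt is a gameplay ability that launches a fire bolt projectile toward the point under the mouse cursor.
; A target data task supplies the hit location, which is passed to the avatar through a message before the fire bolt montage plays.
; A montage gameplay event then spawns the projectile from the weapon socket at that location, and the ability ends after a short delay.
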(event `self.K2_ActivateAbility`
  (bind (_asynctaskproxy _datahandle) (`TargetDataUnderMouse.CreateTargetDataUnderMouse`)
    (:`ValidData`
      (bind _output_get (set `self.Hit Result Location` (`.Location` (`GameplayStatics.BreakHitResult` (`AbilitySystemBlueprintLibrary.GetHitResultFromTargetData` _datahandle)))))
      (message `CombotInterface.PassTargetDataVector` (`self.GetAvatarActorFromActorInfo`) _output_get)
      (`AbilityTask_PlayMontageAndWait.CreatePlayMontageAndWaitProxy` "None" "/Game/BluePrint/Character/Aura/Animotion/AnimotionMontage/AM_FireBolt.AM_FireBolt" 1.0 "None" false
        (:`then`
          (`AbilityTask_WaitGameplayEvent.WaitGameplayEvent` (struct :`TagName` "Event.Montage.FireBolt") null
            (:`EventReceived`
              (`self.SpawnProjectile` (`self.Hit Result Location`) (`BlueprintGameplayTagLibrary.MakeLiteralGameplayTag` (struct :`TagName` "CombatSocket.Weapon")))
              (`KismetSystemLibrary.Delay` 0.5)
              (`self.K2_EndAbility`))))))))