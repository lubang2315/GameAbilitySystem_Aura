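; BP_FireBolt is the Fire Bolt projectile actor, with a fallback that removes bolts left lingering after missing an already-dead target.
; Each Tick it compares its current location with the previous one and treats movement below MinLength as stalled.
; A stalled bolt plays the impact sound, spawns a Niagara fire explosion at its location and destroys itself.
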(event `self.ReceiveTick`
  (params (DeltaSeconds :type "Float (single-precision)"))
  ;[1 1 1] Enemy Already dead The fireball may miss the target but will not disappear
  (set `self.LastLocation` (`self.NewLocation`))
  (set `self.NewLocation` (`self.K2_GetActorLocation`))
  (if (< (`KismetMathLibrary.VSize` (- (`self.NewLocation`) (`self.LastLocation`))) (`self.MinLength`))
    (`GameplayStatics.PlaySoundAtLocation` "/Game/Assets/Sounds/Abilities/FireBolt/sfx_FireBolt_Impact.sfx_FireBolt_Impact" (`self.NewLocation`) (struct) 1.0 1.0 0.0 null null null null)
    (`NiagaraFunctionLibrary.SpawnSystemAtLocation` "/Game/Assets/Effects/Projectiles/FireExplosion/NS_FireExplosion1.NS_FireExplosion1" (`self.NewLocation`))
    (`self.K2_DestroyActor`)))

(fn `UserConstructionScript`)