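; GAS ability for Electrocute, a channeled lightning beam cast at the target under the mouse.
; After a montage event it locks movement and adds ShockLoop cues, chaining to additional targets when the hit actor implements the combat interface.
; A looping timer commits cost and applies SetByCaller lightning damage to each target.
; Input release, after a minimum active time, removes cues and commits cooldown; target-death handlers also clean up beams.
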(event `self.K2_ActivateAbility`
  ;[1 1 1] Is implement CombatInterface?
  (if (`KismetSystemLibrary.DoesImplementInterface` (`self.GetAvatarActorFromActorInfo`) "/Script/Aura_End.CombotInterface")
    ;[1 1 1] Get UnderMouse Info and Store Local Variable
    (bind (_asynctaskproxy _datahandle) (`TargetDataUnderMouse.CreateTargetDataUnderMouse`)
      (:`ValidData`
        (`self.StoreMouseDataInfo` (`AbilitySystemBlueprintLibrary.GetHitResultFromTargetData` _datahandle))
        (`self.StoreOwnerVariables`)
        (`|ExecutionSequence`
          (:`then_0`
            (set `PlayerController.bShowMouseCursor` false (`self.OwnerPlayerController`))
            ;[1 1 1] pass Montage Enemy Location and turn
            (message `CombotInterface.PassTargetDataVector` (`self.GetAvatarActorFromActorInfo`) (`self.MouseHitLocation`))
            ;[1 1 1] Use GameplayCue play Sound
            (`self.K2_ExecuteGameplayCue` (struct :`TagName` "GameplayCue.Shockbrust"))
            (`AbilityTask_PlayMontageAndWait.CreatePlayMontageAndWaitProxy` "None" (`self.Montage_Electorcute`)
              (:`then`
                (`AbilityTask_WaitGameplayEvent.WaitGameplayEvent` (struct :`TagName` "Event.Montage.Electorcute") null true ; 这里不直接使用前面播放蒙太奇的Complement节点主要是施法循环动画的衔接
                  (:`EventReceived`
                    (message `CombotInterface.SetInShockLoop` (`self.GetAvatarActorFromActorInfo`) true)
                    (`CharacterMovementComponent.DisableMovement` (`Character.CharacterMovement` (`self.OwnerCharacter`)))
                    (`self.Use Gameplay Cue Play Electric Beam`)
                    (bind _returnvalue (`KismetSystemLibrary.K2_SetTimerDelegate` (delegate `Apply Damage And Cost`) (`self.ApplycationDamagetInterval`) true))
                    (set `self.Timer by Event ` _returnvalue))))))
          (:`then_1`
            (bind (_asynctaskproxy_2 _timeheld) (`AbilityTask_WaitInputRelease.WaitInputRelease` false)
              (:`OnRelease`
                (bind _output_get (set `self.Time Held` _timeheld))
                (if (< _output_get (`self.MinActiveTime`))
                  (`KismetSystemLibrary.Delay` (- (`self.MinActiveTime`) (`self.Time Held`))))
                (`self.PrepareToEndAbility`)
                (`self.Remove All Gameplay Cue`)
                (`self.Clear Timer And End Ability`)))))))
    (else
      (`self.K2_EndAbility`))))

(event `Apply Damage And Cost`
  (bind _returnvalue (`self.K2_CommitAbilityCost` false))
  (if _returnvalue
    (`self.ApplyDamage`)
    (else
      (`KismetSystemLibrary.K2_ClearAndInvalidateTimerHandle` (`self.Timer by Event `))
      (`self.K2_EndAbility`))))

(event `self.PrimaryTargetDied`
  (params (DeadActor :type "Actor Object Reference"))
  (`GameplayCueFunctionLibrary.RemoveGameplayCueOnActor` DeadActor (struct :`TagName` "GameplayCue.ShockLoop") (`self.GameplayCueParameters`))
  (for _array_element (`self.Out Additional Target`)
    (`self.RemoveActorGameplayCue` _array_element)
    (`self.PrepareToEndAbility`)
    (`self.Clear Timer And End Ability`))
  (`BlueprintMapLibrary.Map_Clear` (`self.AdditionalActorsToCueParameters`)))

(event `self.AdditionalTargetDied`
  (params (DeadActor :type "Actor Object Reference"))
  (`self.RemoveActorGameplayCue` DeadActor)
  (`KismetArrayLibrary.Array_RemoveItem` (`self.Out Additional Target`) DeadActor))

(fn `ApplyActorDamage`
  (params (Actor :type "Actor Object Reference"))
  (bind _returnvalue (`self.GetAbilitySystemComponentFromActorInfo`))
  (bind _output_get (set `self.Tareget ASC` (`AbilitySystemBlueprintLibrary.GetAbilitySystemComponent` Actor)))
  (if (`KismetSystemLibrary.IsValid` _output_get)
    (bind _output_get_2 (set `self.Gameplay Spec` (`AbilitySystemComponent.MakeOutgoingSpec` _returnvalue (`self.DamageEffectClass`) (`KismetMathLibrary.Conv_IntToDouble` (`self.GetAbilityLevel`)) (`AbilitySystemComponent.MakeEffectContext` _returnvalue))))
    (`AbilitySystemBlueprintLibrary.AssignTagSetByCallerMagnitude` _output_get_2 (struct :`TagName` "Damage.Lightning") (`self.GetDamageAtLevel`))
    (`AbilitySystemComponent.BP_ApplyGameplayEffectSpecToSelf` (`self.Tareget ASC`) (`self.Gameplay Spec`))))

(fn `ApplyDamage`
  (`self.ApplyActorDamage` (`self.MouseHitActor`))
  (for _array_element (`self.Out Additional Target`)
    (`self.ApplyActorDamage` _array_element)))

(fn `Clear Timer And End Ability`
  (`self.K2_CommitAbilityCooldown` false)
  (`KismetSystemLibrary.K2_ClearAndInvalidateTimerHandle` (`self.Timer by Event `))
  (`self.K2_EndAbility`))

(fn `PrepareToEndAbility`
  (message `CombotInterface.SetInShockLoop` (`self.GetAvatarActorFromActorInfo`) false)
  (set `PlayerController.bShowMouseCursor` true (`self.OwnerPlayerController`))
  (`CharacterMovementComponent.SetMovementMode` (`Character.CharacterMovement` (`self.OwnerCharacter`)) "MOVE_Walking" 0) ; 有直接设置禁用移动组件的，但是没有直接启用的，但是可以通过设置运动模式启用
)

(fn `Remove All Gameplay Cue`
  (if (`self.IsImplementInterFace`)
    (`GameplayCueFunctionLibrary.RemoveGameplayCueOnActor` (`self.MouseHitActor`) (struct :`TagName` "GameplayCue.ShockLoop") (`self.GameplayCueParameters`))
    (else
      (`GameplayCueFunctionLibrary.RemoveGameplayCueOnActor` (`self.GetAvatarActorFromActorInfo`) (struct :`TagName` "GameplayCue.ShockLoop") (`self.GameplayCueParameters`))))
  (for _array_element (`self.Out Additional Target`)
    (`self.RemoveActorGameplayCue` _array_element))
  (`BlueprintMapLibrary.Map_Clear` (`self.AdditionalActorsToCueParameters`)))

(fn `RemoveActorGameplayCue`
  (params (Target :type "Actor Object Reference"))
  (bind (_value _returnvalue) (`BlueprintMapLibrary.Map_Find` (`self.AdditionalActorsToCueParameters`) Target))
  (set `self.ClealActorCueParameters` _value)
  (if _returnvalue
    (`GameplayCueFunctionLibrary.RemoveGameplayCueOnActor` Target (struct :`TagName` "GameplayCue.ShockLoop") (`self.ClealActorCueParameters`))))

(fn `Use Gameplay Cue Play Electric Beam`
  (bind _array_element (`self.Array Element`))
  (`self.TraceFirstTarget` (`self.MouseHitLocation`))
  (bind _returnvalue (message `CombotInterface.GetWeapon` (`self.GetAvatarActorFromActorInfo`)))
  (set `self.GameplayCueParameters` (`AbilitySystemBlueprintLibrary.MakeGameplayCueParameters` 0.0 0.0 (struct) (struct) (struct) (struct) (struct) (`self.MouseHitLocation`) (0.0 0.0 0.0) null null (`self.MouseHitActor`) null 1 1 _returnvalue))
  (bind _output_get (set `self.IsImplementInterFace` (`KismetSystemLibrary.DoesImplementInterface` (`self.MouseHitActor`) "/Script/Aura_End.CombotInterface")))
  (if _output_get
    (set `self.Cue Target` (`self.MouseHitActor`))
    (else
      (set `self.Cue Target` (`self.GetAvatarActorFromActorInfo`))))
  (`GameplayCueFunctionLibrary.AddGameplayCueOnActor` (`self.Cue Target`) (struct :`TagName` "GameplayCue.ShockLoop") (`self.GameplayCueParameters`))
  (if (`self.IsImplementInterFace`)
    (bind _outadditionaltarget (`self.StoreAdditionalTarget`))
    (bind _output_get_2 (set `self.Out Additional Target` _outadditionaltarget))
    (for _array_element_2 _output_get_2
      (set `self.Array Element` _array_element_2)
      (bind _output_get_3 (set `self.Enemy GameplayCue Para` (`AbilitySystemBlueprintLibrary.MakeGameplayCueParameters` 0.0 0.0 (struct) (struct) (struct) (struct) (struct) (`Actor.K2_GetActorLocation` _array_element) (0.0 0.0 0.0) null null _array_element null 1 1 (`Actor.RootComponent` (`self.MouseHitActor`)))))
      (`BlueprintMapLibrary.Map_Add` (`self.AdditionalActorsToCueParameters`) (`self.Array Element`) _output_get_3)
      (`GameplayCueFunctionLibrary.AddGameplayCueOnActor` (`self.Array Element`) (struct :`TagName` "GameplayCue.ShockLoop") (`self.Enemy GameplayCue Para`)))))