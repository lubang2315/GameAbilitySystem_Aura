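; Gameplay Ability for the Arcane Shards spell, which strikes a series of ground points around a mouse-targeted location with radial damage.
; After a cost check, it shows a magic circle, awaits a press, then gets randomly rotated points from a spawned BP_PointsCollection.
; A montage event starts a looping timer that, per point, damages nearby live players with outward knockback and fires a GameplayCue.
; Cost commits at that event, cooldown after the last shard.
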(event `self.K2_ActivateAbility`
  (bind _returnvalue (`self.GetArcaneShardsNum`))
  (bind _returnvalue_2 (`self.K2_CheckAbilityCost`))
  (if _returnvalue_2
    (`|ExecutionSequence`
      (:`then_0`
        (message `PlayerInterface.ShowMagicCircle` (`self.GetAvatarActorFromActorInfo`) null))
      (:`then_1`
        (`AbilityTask_WaitInputPress.WaitInputPress` false
          (:`OnPress`
            (bind (_asynctaskproxy _datahandle) (`TargetDataUnderMouse.CreateTargetDataUnderMouse`)
              (:`ValidData`
                (bind _output_get (set `self.Impact Point` (`.ImpactPoint` (`GameplayStatics.BreakHitResult` (`AbilitySystemBlueprintLibrary.GetHitResultFromTargetData` _datahandle)))))
                (bind _returnvalue_3 (`|SpawnActorFromClass` "/Game/BluePrint/Actor/PointsCollection/BP_PointsCollection.BP_PointsCollection_C" (`KismetMathLibrary.MakeTransform` _output_get) "AlwaysSpawn" "MultiplyWithRoot" null null))
                (bind _output_get_2 (set `self.PointCollection` _returnvalue_3))
                (`KismetSystemLibrary.PrintString` (`KismetStringLibrary.Conv_IntToString` _returnvalue))
                (set `self.TArryPoints` (`PointCollection.GetGroundPoints` _output_get_2 (`self.Impact Point`) _returnvalue (`KismetMathLibrary.RandomFloatInRange` 0.0 360.0)))
                (message `CombotInterface.PassTargetDataVector` (`self.GetAvatarActorFromActorInfo`) (`self.Impact Point`))
                (`AbilityTask_PlayMontageAndWait.CreatePlayMontageAndWaitProxy` "None" "/Game/BluePrint/GAS/GA/GA_Aura/Arcane/AM_ArcaneShards.AM_ArcaneShards"
                  (:`then`
                    (`AbilityTask_WaitGameplayEvent.WaitGameplayEvent` (struct :`TagName` "Event.Montage.ArcaneShards") null
                      (:`EventReceived`
                        (`KismetSystemLibrary.K2_SetTimerDelegate` (delegate `Spawn Shard`) (`self.Time`) true false -0.2)
                        (message `PlayerInterface.HideMagicCircle` (`self.GetAvatarActorFromActorInfo`))
                        (`self.K2_CommitAbilityCost` false)))))))))))))

(event `Spawn Shard`
  (bind _returnvalue (`self.GetAvatarActorFromActorInfo`))
  (if (< (`self.PointsCount`) (`self.GetArcaneShardsNum`))
    (set `self.PointLocation` (`SceneComponent.K2_GetComponentLocation` (`|GetArrayItem` (`self.TArryPoints`) (`self.PointsCount`))))
    (bind _outoverlappingactors (`MyFunctionLibrary.GetLivePlayersWithinRadius` _returnvalue (`self.RadialDamageOuterRadius`) (`|MakeArray` _returnvalue) (`self.PointLocation`)))
    (bind _output_get (set `self.Out Overlapping Actors` _outoverlappingactors))
    (for _array_element _output_get
      (bind _returnvalue_2 (- (`Actor.K2_GetActorLocation` _array_element) (`self.PointLocation`)))
      (`MyFunctionLibrary.ApplyGameplayEffect` (`self.MakeDamageEffectPramsFromClassDefault` _array_element (`self.PointLocation`) true _returnvalue_2 true _returnvalue_2 true 45.0)))
    (`/Engine/EditorBlueprintResources/StandardMacros.IncrementInt` (`self.PointsCount`)
      (:`  `
        (`self.K2_ExecuteGameplayCueWithParams` (struct :`TagName` "GameplayCue.ArcaneShader") (`AbilitySystemBlueprintLibrary.MakeGameplayCueParameters` 0.0 0.0 (struct) (struct) (struct) (struct) (struct) (`self.PointLocation`)))))
    (else
      (`KismetSystemLibrary.Delay` 0.2)
      (`self.K2_CommitAbilityCooldown` false)
      (`self.K2_EndAbility`)
      (`KismetSystemLibrary.PrintString` "Hello"))))

(event `self.K2_OnEndAbility`
  (params (bWasCancelled :type Boolean)))