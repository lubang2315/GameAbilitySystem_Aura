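; Enemy ranged attack Gameplay Ability that fires a projectile at the avatar's current combat target.
; On activation it passes the target's location to the avatar through the combat interface, then plays a randomly picked tagged montage.
; The montage's tag gameplay event triggers SpawnProjectile at the target's re-read location, so the shot follows animation timing.
; The ability ends when the montage completes, blends out, is interrupted or cancelled, or when the interface cast fails.
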(event `self.K2_ActivateAbility`
  (bind _returnvalue (`self.GetAvatarActorFromActorInfo`))
  (bind _returnvalue_2 (`self.GetAvatarActorFromActorInfo`))
  (bind _returnvalue_3 (message `EnemyInterface.GetCombotTarget` _returnvalue))
  (bind _ascombot_interface (cast `CombotInterface` _returnvalue)
    (:`then`
      (`CombotInterface.PassTargetDataVector` _ascombot_interface (`Actor.K2_GetActorLocation` _returnvalue_3))
      (bind _returnvalue_4 (message `CombotInterface.GetTaggedMontages` _returnvalue))
      (bind _output_get (set `self.TaggedMontage` (`self.GetRandomTaggedMontageFromArray` _returnvalue_4)))
      (bind (_montage _montagetag) (break `TaggedMontage` _output_get))
      (`AbilityTask_PlayMontageAndWait.CreatePlayMontageAndWaitProxy` "None" _montage 1.0 "None" false
        (:`then`
          (`AbilityTask_WaitGameplayEvent.WaitGameplayEvent` _montagetag null
            (:`EventReceived`
              (message `CombotInterface.GetCombatSocketLocation` _returnvalue_2 _montagetag)
              (bind _returnvalue_5 (message `EnemyInterface.GetCombotTarget` _returnvalue_2))
              (`self.SpawnProjectile` (`Actor.K2_GetActorLocation` _returnvalue_5)))))
        (:`OnCompleted`
          (`self.K2_EndAbility` :!label _label))
        (:`OnBlendOut`
          (goto _label))
        (:`OnInterrupted`
          (goto _label))
        (:`OnCancelled`
          (goto _label))))
    (:`CastFailed`
      (`self.K2_EndAbility`))))