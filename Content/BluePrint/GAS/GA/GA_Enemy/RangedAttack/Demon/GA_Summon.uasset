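; Gameplay ability for a demon enemy that summons random minions around it.
; On activation it shuffles computed spawn locations, marks each with a ground Niagara effect, and plays the summon montage.
; A montage gameplay event then starts a delayed loop that spawns one random minion per location in turn, slightly raised and facing away from the caster.
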(event `self.K2_ActivateAbility`
  ;[1 1 1] 创建召唤敌人生成位置
  (bind _returnvalue (`self.GetSpawnLocations`))
  (bind _output_get (set `self.SpawnLocation` _returnvalue))
  (`KismetArrayLibrary.Array_Shuffle` _output_get)
  (for _array_element _output_get
    ;[1 1 1] 通过特效让玩家知道即将召唤敌人位置
    (`NiagaraFunctionLibrary.SpawnSystemAtLocation` "/Game/Assets/Effects/Combat/NS_GroundSummon.NS_GroundSummon" _array_element))
  ;[1 1 1] 播放召唤动画并等待触发通知
  (`AbilityTask_PlayMontageAndWait.CreatePlayMontageAndWaitProxy` "None" "/Game/BluePrint/Character/Enemy/Shaman/Animoation/AM_Summons.AM_Summons"
    (:`then`
      (`AbilityTask_WaitGameplayEvent.WaitGameplayEvent` (struct :`TagName` "Montage.Attack.1") null
        (:`EventReceived`
          (`self.Spawn Enemy`))))))

(event `Spawn Enemy`
  (bind _returnvalue (+ (`|GetArrayItem` (`self.SpawnLocation`) (`self.SpawnLocationIndex`)) (0.0 0.0 70.0)))
  ;[1 1 1] 随机生成召唤敌人
  (if (< (`self.SpawnLocationIndex`) (`KismetArrayLibrary.Array_Length` (`self.SpawnLocation`))) :!label _label
    (`|SpawnActorFromClass` (`self.GetRandomMinionsClass`) (`KismetMathLibrary.MakeTransform` _returnvalue (`KismetMathLibrary.FindLookAtRotation` (`Actor.K2_GetActorLocation` (`self.GetAvatarActorFromActorInfo`)) _returnvalue)) "AlwaysSpawn" "MultiplyWithRoot" null null)
    (`/Engine/EditorBlueprintResources/StandardMacros.IncrementInt` (`self.SpawnLocationIndex`)
      (:`  `
        (`KismetSystemLibrary.Delay` 0.2)
        (goto _label)))))