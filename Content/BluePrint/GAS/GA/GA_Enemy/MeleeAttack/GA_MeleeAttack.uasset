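; Enemy melee Gameplay Ability that turns toward the combat target and plays a random tagged attack montage.
; The target's location goes through CombotInterface, and the montage's gameplay event triggers a small radius check at its tagged socket.
; Non-friendly live players found there take damage, and any hit fires a MeleeImpact cue at the stored target location.
; The ability ends on a miss or montage exit, without stopping the montage.
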(event `self.K2_ActivateAbility`
  (set `self.HasHitTag` false)
  (`self.Turning Target`))

(event `Turning Target`
  (bind _returnvalue (`self.GetAvatarActorFromActorInfo`))
  (bind _returnvalue_2 (message `EnemyInterface.GetCombotTarget` _returnvalue))
  (bind _ascombot_interface (cast `CombotInterface` _returnvalue)
    (:`then`
      (bind _returnvalue_3 (`Actor.K2_GetActorLocation` _returnvalue_2))
      (set `self.WeaponHitLocation` _returnvalue_3)
      (`CombotInterface.PassTargetDataVector` _ascombot_interface _returnvalue_3)
      (`self.Play montage About GA`))
    (:`CastFailed`
      (`self.K2_EndAbility`))))

(event `Play montage About GA`
  (bind _returnvalue (message `CombotInterface.GetTaggedMontages` (`self.GetAvatarActorFromActorInfo`)))
  (bind _output_get (set `self.TaggedMontage` (`self.GetRandomTaggedMontageFromArray` _returnvalue)))
  (`|ExecutionSequence`
    (:`then_0`
      (bind (_montage _montagetag _sockettag) (break `TaggedMontage` _output_get))
      (set `self.Montage` _montage)
      (set `self.Montage Tag` _montagetag)
      (set `self.Socket Tag` _sockettag))
    (:`then_1`
      (`AbilityTask_PlayMontageAndWait.CreatePlayMontageAndWaitProxy` "None" (`self.Montage`) 1.0 "None" false
        (:`then`
          (`self.Activate Cue`))
        (:`OnCompleted`
          (`self.K2_EndAbility` :!label _label))
        (:`OnBlendOut`
          (goto _label))
        (:`OnInterrupted`
          (goto _label))
        (:`OnCancelled`
          (goto _label))))))

(event `Activate Cue`
  (bind _returnvalue (`self.GetAvatarActorFromActorInfo`))
  (`AbilityTask_WaitGameplayEvent.WaitGameplayEvent` (`self.Montage Tag`) null
    (:`EventReceived`
      (bind _returnvalue_2 (message `CombotInterface.GetCombatSocketLocation` _returnvalue (`self.Socket Tag`)))
      (bind _outoverlappingactors (`MyFunctionLibrary.GetLivePlayersWithinRadius` _returnvalue 30.0 (`|MakeArray` (`self.GetAvatarActorFromActorInfo`)) _returnvalue_2))
      (for _array_element _outoverlappingactors
        (if (`MyFunctionLibrary.ISNotFriend` _array_element (`self.GetAvatarActorFromActorInfo`))
          (`self.CauseDamage` _array_element)
          (set `self.HasHitTag` true)))
      (if (`self.HasHitTag`)
        (`self.K2_ExecuteGameplayCueWithParams` (struct :`TagName` "GameplayCue.MeleeImpact") (`AbilitySystemBlueprintLibrary.MakeGameplayCueParameters` 0.0 0.0 (struct) (struct) (struct) (`BlueprintGameplayTagLibrary.MakeGameplayTagContainerFromTag` (`.MontageTag` (break `TaggedMontage` (`self.TaggedMontage`)))) (struct) (`self.WeaponHitLocation`) (0.0 0.0 0.0) null (`self.GetAvatarActorFromActorInfo`) _array_element))
        (else
          (`self.K2_EndAbility`))))))