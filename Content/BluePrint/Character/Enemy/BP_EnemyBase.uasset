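; Base enemy Blueprint handling motion-warp facing, spawn-in scaling, death dissolve and loot drops.
; Timelines optionally grow the mesh on BeginPlay and drive the Dissolve parameter on body and weapon materials.
; SpawnLoot gets tiered items and evenly spaced rotators, then a looping timer spawns them around the enemy at randomized distances.
; Level-override items receive the player's level, and only that branch advances the index that ends the timer.
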(event `CombotInterface.PassTargetDataVector`
  (params (Vector :type "Vector Structure (by ref)"))
  (`MotionWarpingComponent.AddOrUpdateWarpTargetFromLocation` (`self.MotionWarping`) "FacingTarget" Vector))

(event `self.StartDissolveTimeline`
  (params (DynamicMaterialInstance :type "MaterialInstanceDynamic Object Reference"))
  ;[1 1 1] Die DIssolve
  (bind (_direction `_新建轨道_0`) (`Timeline|时间轴`)
    (:`Update`
      (`MaterialInstanceDynamic.SetScalarParameterValue` DynamicMaterialInstance "Dissolve" `_新建轨道_0`))))

(event `self.WeaponStartDissolveTimeline`
  (params (DynamicMaterialInstance :type "MaterialInstanceDynamic Object Reference"))
  ;[1 1 1] Die DIssolve
  (bind (_direction `_新建轨道_0`) (`Timeline|时间轴_0`)
    (:`Update`
      (`MaterialInstanceDynamic.SetScalarParameterValue` DynamicMaterialInstance "Dissolve" `_新建轨道_0`))))

(event `self.ReceiveBeginPlay`
  (if (`self.Chrarcter Generation Effect`)
    (bind (_direction `_新建轨道_0`) (`Timeline|时间轴_1`)
      (:`Update`
        (`SceneComponent.SetRelativeScale3D` (`self.Mesh`) (`KismetMathLibrary.MakeVector` `_新建轨道_0` `_新建轨道_0` `_新建轨道_0`))))))

(event `self.SpawnLoot`
  (bind _returnvalue (`MyFunctionLibrary.GetLootTiers` null))
  (`/Engine/EditorBlueprintResources/StandardMacros.IsValid` _returnvalue
    (:`Is Valid`
      (bind _returnvalue_2 (`LootTiers.GetLootItems` _returnvalue))
      (set `self.LootTiers` _returnvalue_2)
      (bind _returnvalue_3 (`MyFunctionLibrary.EvenlySpacedRotators` (`self.GetActorForwardVector`) (`KismetMathLibrary.Vector_Up`) 360.0 (`KismetArrayLibrary.Array_Length` _returnvalue_2)))
      (set `self.SpawnLootLoaction` _returnvalue_3)
      (`self.SpawningLootTiers`))))

(event `SpawningLootTiers`
  (set `self.SpawnLootCount` 0)
  (bind _returnvalue (`KismetSystemLibrary.K2_SetTimerDelegate` (delegate `SpawnLootTiers`) 0.1 true))
  (set `self.TimerHandle` _returnvalue)
  (`self.SpawnLootTiers`))

(event `SpawnLootTiers`
  (bind _output (`|GetArrayItem` (`self.SpawnLootLoaction`) (`self.SpawnLootCount`)))
  (bind (_lootitemclass _blootleveloverride) (break `LootItem` (`|GetArrayItem` (`self.LootTiers`) (`self.SpawnLootCount`))))
  (bind (_returnvalue_x _returnvalue_y) (`KismetMathLibrary.BreakVector` (+ (* (`KismetMathLibrary.GetForwardVector` _output) (`KismetMathLibrary.RandomFloatInRange` 80.0 50.0)) (`self.K2_GetActorLocation`))))
  (bind _returnvalue (`|SpawnActorFromClass` _lootitemclass (`KismetMathLibrary.MakeTransform` (`KismetMathLibrary.MakeVector` _returnvalue_x _returnvalue_y 50.0) _output) "Undefined" "MultiplyWithRoot" null null))
  (if _blootleveloverride
    (`self.SetLootTiresLevel` _returnvalue)
    (`self.ClearTimerHandle`)))

(event `SetLootTiresLevel`
  (params (SpawnActor :type "Actor Object Reference"))
  (bind _asbp_tool_actor_base (cast `/Game/BluePrint/Actor/RecoverHP/BP_ToolActorBase` SpawnActor))
  (`/Engine/EditorBlueprintResources/StandardMacros.IsValid` _asbp_tool_actor_base
    (:`Is Valid`
      (bind _returnvalue (`CombotInterface.GetPlayerLevel`))
      (set `MyActor.ActorLever` (`KismetMathLibrary.Conv_IntToDouble` _returnvalue) _asbp_tool_actor_base))))

(event `ClearTimerHandle`
  (bind _result (`/Engine/EditorBlueprintResources/StandardMacros.IncrementInt` (`self.SpawnLootCount`))
    (:`  `
      (if (>= _result (`KismetArrayLibrary.Array_Length` (`self.LootTiers`)))
        (`KismetSystemLibrary.K2_ClearAndInvalidateTimerHandle` (`self.TimerHandle`))))))

(fn `UserConstructionScript`)