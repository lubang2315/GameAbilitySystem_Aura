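; BP_ToolActorBase is a tool item actor, apparently a base for HP recovery pickups, with animated spawn, idle motion and sound cues.
; On BeginPlay it plays a sound and a timeline drives height and scale, with a one-shot sound when elevation dips below zero.
; When the timeline finishes it starts rotation and sinusoidal movement.
; Tick applies CalculatedLocation and CalculatedRotation, which are computed outside these graphs, and destruction plays a third sound.
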(event `self.ReceiveBeginPlay`
  (bind (_calculatedlocation_x _calculatedlocation_y _calculatedlocation_z) (`KismetMathLibrary.BreakVector` (`self.CalculatedLocation`)))
  (`GameplayStatics.PlaySoundAtLocation` (`self.Sound1`) (`self.K2_GetActorLocation`) (struct) 1.0 1.0 0.0 null null null null)
  (bind (_direction _elevation _scale) (`Timeline|时间轴`)
    (:`Update`
      (set `self.Elevation` _elevation)
      (`self.K2_SetActorLocation` (`KismetMathLibrary.MakeVector` _calculatedlocation_x _calculatedlocation_y (+ _calculatedlocation_z (* _elevation 130.0))))
      (`self.SetActorScale3D` (`KismetMathLibrary.MakeVector` _scale _scale _scale))
      (if (<= (`self.Elevation`) -0.02)
        (`/Engine/EditorBlueprintResources/StandardMacros.DoOnce` false
          (:`Completed`
            (`GameplayStatics.PlaySoundAtLocation` (`self.Sound2`) (`self.K2_GetActorLocation`) (struct) 1.0 1.0 0.0 null null null null)))))
    (:`Finished`
      (`self.StartRotation`)
      (`self.StartSinusoidalMovement`))))

(event `self.ReceiveTick`
  (params (DeltaSeconds :type "Float (single-precision)"))
  (`self.K2_SetActorLocation` (`self.CalculatedLocation`))
  (`self.K2_SetActorRotation` (`self.CalculatedRotation`)))

(event `self.ReceiveDestroyed`
  (`GameplayStatics.PlaySoundAtLocation` (`self.Sound3`) (`self.K2_GetActorLocation`) (struct) 1.0 1.0 0.0 null null null null))

(fn `UserConstructionScript`)