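; BP_FireBlast is a fire skill actor that flies forward, returns to ReturnToActor and explodes.
; On the server, two chained timelines lerp it out by SkillDistance, then back toward the target's live location.
; Within DeatoryDistance, it plays its impact and applies radial explosion damage through GAS to nearby live players, excluding the owner, with angled-up knockback and death impulse, then destroys itself.
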(event `self.StartOutgoingTimeline`
  (bind _returnvalue (`self.GetOwner`))
  (bind _array (`|MakeArray` _returnvalue))
  (`/Engine/EditorBlueprintResources/ActorMacros.Switch Has Authority`
    (:`Authority`
      (set `self.ActorLocation` (`self.K2_GetActorLocation`))
      (set `self.FinishDiatance` (+ (`self.ActorLocation`) (* (`self.GetActorForwardVector`) (`self.Skill Distance`))))
      (bind (_direction _outgoing_track) (`Timeline|OutgoingTimeline`)
        (:`Update`
          (`self.K2_SetActorLocation` (`KismetMathLibrary.VLerp` (`self.ActorLocation`) (`self.FinishDiatance`) _outgoing_track)))
        (:`Finished`
          (bind (_direction_2 _outgoing_track_2) (`Timeline|时间轴`)
            (:`Update`
              (bind _output_get (set `self.FinishActorLocation` (`self.K2_GetActorLocation` (`self.ReturnToActor`))))
              (`self.K2_SetActorLocation` (`KismetMathLibrary.VLerp` (`self.FinishDiatance`) _output_get _outgoing_track_2))
              (if (<= (`KismetMathLibrary.Vector_Distance` (`self.K2_GetActorLocation`) (`self.FinishActorLocation`)) (`self.DeatoryDistance`))
                (`self.PlayImpact`)
                (`MyFunctionLibrary.SetIsRadialDamageEffectParams` (`self.ExplosionDamageParams`) true (`self.Inner Radius`) (`self.Out Radius`) (`self.K2_GetActorLocation`))
                (`KismetArrayLibrary.Array_Add` _array self)
                (bind _outoverlappingactors (`MyFunctionLibrary.GetLivePlayersWithinRadius` _returnvalue (`self.Out Radius`) _array (`self.K2_GetActorLocation`)))
                (bind _output_get_2 (set `self.Out Overlapping Actors` _outoverlappingactors))
                (for _array_element _output_get_2
                  (bind _output_get_3 (set `self.Array Element` _array_element))
                  (bind _returnvalue_2 (`AbilitySystemBlueprintLibrary.GetAbilitySystemComponent` _output_get_3))
                  (`MyFunctionLibrary.SetEffectParamsTargetASC` (`self.ExplosionDamageParams`) _returnvalue_2)
                  (if (`KismetSystemLibrary.IsValid` _returnvalue_2)
                    (bind _output_get_4 (set `self.Attack Derction` (- (`self.K2_GetActorLocation` (`self.Array Element`)) (`self.K2_GetActorLocation`))))
                    (bind (_returnvalue_roll _returnvalue_pitch _returnvalue_yaw) (`KismetMathLibrary.BreakRotator` (`KismetMathLibrary.MakeRotFromX` _output_get_4)))
                    (bind _output_get_5 (set `self.Attack Derction` (`KismetMathLibrary.GetForwardVector` (`KismetMathLibrary.MakeRotator` _returnvalue_roll 45.0 _returnvalue_yaw))))
                    (`MyFunctionLibrary.SetKnockbackDirection` (`self.ExplosionDamageParams`) _output_get_5 700.0)
                    (`MyFunctionLibrary.SetDeathImpulseDirection` (`self.ExplosionDamageParams`) (`self.Attack Derction`) 700.0)
                    (`MyFunctionLibrary.ApplyGameplayEffect` (`self.ExplosionDamageParams`))
                    (`self.K2_DestroyActor`)))
                (`self.K2_DestroyActor`)))))))))

(fn `UserConstructionScript`)