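; BP_FadeActor is an actor whose mesh fades out and back in through a material parameter.
; Construction caches original materials and builds dynamic instances from FadeMaterialInstance.
; FadeOut swaps those instances in and plays a timeline driving their "Fade" scalar; Fadein reverses it.
; On finish, zero fade ignores GameTraceChannel2, while full fade restores original materials and blocking; BlockVisible extends both collision changes to Visibility.
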(event `/Game/BluePrint/Actor/FadeActor/FadeInterFace/BI_FadeMaterialInstance.FadeOut`
  (`self.SetFadeMaterialInstanceByMesh`)
  (bind (_direction _fadetime) (`Timeline|时间轴` :!label _label)
    (:`Update`
      (for _array_element (`self.DynamicMaterialInstance`)
        (`MaterialInstanceDynamic.SetScalarParameterValue` _array_element "Fade" _fadetime)))
    (:`Finished`
      (if (>= _fadetime 1.0)
        (for (_array_element_2 _array_index) (`self.OriginalMaterial`)
          (`PrimitiveComponent.SetMaterial` (`self.Mesh`) _array_index _array_element_2)
          (`PrimitiveComponent.SetCollisionResponseToChannel` (`self.Mesh`) "ECC_GameTraceChannel2" "ECR_Block")
          (if (`self.BlockVisible`)
            (`PrimitiveComponent.SetCollisionResponseToChannel` (`self.Mesh`) "ECC_Visibility" "ECR_Block")))
        (elif (<= _fadetime 0.0)
          (`PrimitiveComponent.SetCollisionResponseToChannel` (`self.Mesh`) "ECC_GameTraceChannel2" "ECR_Ignore")
          (if (`self.BlockVisible`)
            (`PrimitiveComponent.SetCollisionResponseToChannel` (`self.Mesh`) "ECC_Visibility" "ECR_Ignore")))))))

(event `/Game/BluePrint/Actor/FadeActor/FadeInterFace/BI_FadeMaterialInstance.FadeIn`
  (goto _label :!via `Reverse`))

(fn `SetFadeMaterialInstanceByMesh`
  (for (_array_element _array_index) (`self.DynamicMaterialInstance`)
    (`PrimitiveComponent.SetMaterial` (`self.Mesh`) _array_index _array_element)))

(fn `UserConstructionScript`
  (`KismetArrayLibrary.Array_Clear` (`self.DynamicMaterialInstance`))
  (set `self.OriginalMaterial` (`MeshComponent.GetMaterials` (`self.Mesh`)))
  (for _array_element (`self.FadeMaterialInstance`)
    (bind _returnvalue (`KismetMaterialLibrary.CreateDynamicMaterialInstance` _array_element))
    (`KismetArrayLibrary.Array_AddUnique` (`self.DynamicMaterialInstance`) _returnvalue)))