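; BP_FlamePillar is a flame pillar actor whose point light changes intensity continuously, apparently to mimic flickering fire.
; On BeginPlay it randomly picks one of two timelines, each driving the light through a float track scaled by the LightIntensity variable.
; When a timeline finishes it triggers another random pick, forming an endless loop of varied light patterns without using Tick.
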(event `self.ReceiveBeginPlay`
  (`self.Random Light`))

(event `Random Light`
  (switch `int` (`KismetMathLibrary.RandomIntegerInRange` 0 1)
    (:`Default`
      (`self.Light Intensity_2` :!label _label))
    (:`0`
      (`self.Light Intensity_1`))
    (:`1`
      (goto _label))))

(event `Light Intensity_1`
  (bind (_direction `_新建轨道_0`) (`Timeline|时间轴` :!via `PlayFromStart`)
    (:`Update`
      (`self.Set Light Intensity` `_新建轨道_0`))
    (:`Finished`
      (`self.Random Light`))))

(event `Light Intensity_2`
  (bind (_direction `_新建轨道_0`) (`Timeline|时间轴_0` :!via `PlayFromStart`)
    (:`Update`
      (`self.Set Light Intensity` `_新建轨道_0`))
    (:`Finished`
      (`self.Random Light`))))

(fn `Set Light Intensity`
  (params (A :type "Float (double-precision)"))
  (`LightComponent.SetIntensity` (`self.PointLight`) (* A (`self.Light Intensity`))))

(fn `UserConstructionScript`)