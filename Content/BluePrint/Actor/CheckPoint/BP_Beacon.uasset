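; BP_Beacon is a checkpoint beacon that lights up when a player first reaches it.
; Overlapping its collision sphere prints a debug string, then actors implementing PlayerInterface set a one-time Reached flag and call HandleGlowEffect, which is defined outside this graph.
; The CheckPointReached event receives a dynamic material instance and plays a timeline that drives its scaled Glow parameter.
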(event `self.CheckPointReached`
  (params (MaterialInstanceDynamic :type "MaterialInstanceDynamic Object Reference"))
  (bind (_direction `_新建轨道_0`) (`Timeline|时间轴`)
    (:`Update`
      (`MaterialInstanceDynamic.SetScalarParameterValue` MaterialInstanceDynamic "Glow" (* `_新建轨道_0` 20.0)))))

(event `self.CheckPointCollisionSphere.OnComponentBeginOverlap`
  (params (OverlappedComponent :type "PrimitiveComponent Object Reference") (OtherActor :type "Actor Object Reference") (OtherComp :type "PrimitiveComponent Object Reference") (OtherBodyIndex :type Integer) (bFromSweep :type Boolean) (SweepResult :type "HitResult Structure (by ref)"))
  (`KismetSystemLibrary.PrintString` "Hello")
  (if (`KismetSystemLibrary.DoesImplementInterface` OtherActor "/Script/Aura_End.PlayerInterface")
    (if (not (`self.bReached`))
      (set `self.bReached` true)
      (`self.HandleGlowEffect`))))

(fn `UserConstructionScript`)